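; Bridge actor that builds a row of wooden planks along an editable spline in the construction script.
; Spline length divided by a clamped MeshLength sets the plank count, and each static mesh component is placed at Index times the unclamped MeshLength along the spline.
; Planks share a fixed rotation, scale and OldWood material, so they do not turn with the curve.
; The event graph has no active logic.
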(event EventBeginPlay)

(event Collision|EventActorBeginOverlap
  (params (OtherActor :type Actor%20Object%20Reference)))

(event EventTick
  (params (DeltaSeconds :type Float%20%28single-precision%29)))

(fn ConstructionScript
  (Utilities|FlowControl|Sequence
    (:then_0
      (Variables|Default|SetLog%20Array (Variables|Default|Getempty))
      (bind _output_get (Variables|Default|SetNumber%20of%20Meshes (/ (Spline|GetSplineLength (Variables|Default|GetBridge)) (Math|Float|Clamp(Float) (Variables|Default|GetMesh%20Length) 1e+02 1e+03))))
      (for _index (range 0 (Math|Float|Truncate _output_get))
        (bind _returnvalue (AddComponent|AddStaticMeshComponent false))
        (bind _returnvalue_2 (Utilities|Array|Add (Variables|Default|GetLog%20Array) _returnvalue))
        (Transformation|SetWorldLocationAndRotation (Utilities|Array|Get(acopy) (Variables|Default|GetLog%20Array) _returnvalue_2) (Spline|GetLocationatDistanceAlongSpline (Variables|Default|GetBridge) (* _index (Variables|Default|GetMesh%20Length)) "World") "-90.000000,0.000000,0.000000" false false)
        (Transformation|SetWorldScale3D _returnvalue "0.200000,4.500000,1.000000")
        (Rendering|Material|SetMaterial _returnvalue 0 "/Game/Materials/OldWood.OldWood")))))