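; Moving deer actor that sways back and forth around its placed position along its right axis.
; The construction script caches the actor's location as the origin and sets mobility to Movable.
; Each Tick sets the location to that origin plus a game-time sine wave, shaped by Speed, Offset and WalkDistance, without sweeping for collision.
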(event EventBeginPlay)

(event Collision|EventActorBeginOverlap
  (params (OtherActor :type Actor%20Object%20Reference)))

(event EventTick
  (params (DeltaSeconds :type Float%20%28single-precision%29))
  (Transformation|SetActorLocation (+ (* (Transformation|GetActorRightVector) (* (Math|Trig|Sin(Radians) (+ (* (Utilities|Time|GetGameTimeinSeconds) (Variables|Default|Getspeed)) (Variables|Default|Getoffset))) (Variables|Default|GetwalkDistance))) (Variables|Default|GetoriginalLocation)) false false))

(fn ConstructionScript
  (Utilities|FlowControl|Sequence
    (:then_0
      (Variables|Default|SetoriginalLocation (Transformation|GetActorLocation)))
    (:then_1
      (Transformation|SetMobility "Movable"))))